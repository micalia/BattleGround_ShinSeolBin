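; Enemy Blueprint for a battleground game that loses health while outside a magnetic zone and keeps its damage widget turned toward the player.
; Any actor overlap beginning or ending toggles the in-zone flag, with no filter on the other actor.
; Tick runs a timer that drains health outside the zone and calls EnemyDieEvent when it runs out.
; Tick also caches the BattleGroundCharacter and yaws the widget to face it.
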(event Collision|EventActorBeginOverlap
  (params (OtherActor :type Actor%20Object%20Reference))
  (Variables|Default|SetIsInMagnetic? true))

(event EventTick
  (params (DeltaSeconds :type Float%20%28single-precision%29))
  (Utilities|FlowControl|Sequence
    (:then_0
      (bind _output_get (Variables|Default|SetmagDamageCurrTime (+ DeltaSeconds (Variables|Default|GetmagDamageCurrTime))))
      (if (> _output_get (Variables|Default|GetmagDamageDelayTime))
        (Variables|Default|SetmagDamageCurrTime 0.0)
        (if (not (Variables|Default|GetIsInMagnetic?))
          (bind _output_get_2 (Variables|Default|SetBP_CurrHP (- (Variables|Default|GetBP_CurrHP) 0.25)))
          (if (not (> _output_get_2 0.0))
            (Class|Enemy|EnemyDieEvent)))))
    (:then_1
      (Utilities|IsValid (Variables|Default|GetPlayerRef)
        (:Is%20Valid
          _)
        (:Is%20Not%20Valid
          (bind _returnvalue (Actor|GetActorOfClass "/Script/BattleGround.BattleGroundCharacter"))
          (Variables|Default|SetPlayerRef _returnvalue)))
      (Transformation|SetWorldRotation (Variables|Default|GetDamageWidget) (Math|Rotator|MakeRotator 0.0 0.0 (.yaw (Math|Rotator|FindLookatRotation (Transformation|GetActorLocation) (Transformation|GetActorLocation (Variables|Default|GetPlayerRef))))) false false))))

(event Collision|EventActorEndOverlap
  (params (OtherActor :type Actor%20Object%20Reference))
  (Variables|Default|SetIsInMagnetic? false))

(event EventBeginPlay
  (Variables|Default|SetBP_CurrHP (Variables|Default|GetFullHp)))

(fn ConstructionScript)