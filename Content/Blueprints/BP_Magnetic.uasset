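; BP_Magnetic is a tall zone actor, apparently a battle-royale style boundary, that spawns at a random XY position and shrinks over the match.
; Tick alternates shrink phases with timed pauses, using thresholds stepped down from GameTime by a fixed term.
; Shrinking steadily reduces XY scale while Z stays fixed, stopping below a minimum.
; That minimum makes the destroy-below-zero check effectively unreachable, and no overlap logic is active.
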(event EventBeginPlay
  (bind _scale (Variables|Default|Getscale))
  (Transformation|SetActorLocation (Math|Vector|MakeVector (Math|Random|RandomFloatinRange -2.741e+04 -1.16e+04) (Math|Random|RandomFloatinRange 2.63e+03 1.444e+04) -4.29e+04) false false)
  (Transformation|SetActorScale3D (Math|Vector|MakeVector _scale _scale 7e+03))
  (Variables|Default|SetnextDelayTime (- (Variables|Default|GetGameTime) (Variables|Default|GetNextDecreaseTermTime))))

(event Collision|EventActorBeginOverlap
  (params (OtherActor :type Actor%20Object%20Reference)))

(event EventTick
  (params (DeltaSeconds :type Float%20%28single-precision%29))
  (if (not (Variables|Default|GetbDelay))
    (bind _output_get (Variables|Default|SetdecreaseCurrTime (+ (Variables|Default|GetdecreaseCurrTime) DeltaSeconds)))
    (if (> (- (Variables|Default|GetGameTime) _output_get) (Variables|Default|GetnextDelayTime))
      (if (not (< (Variables|Default|Getscale) 3e+01))
        (Transformation|SetActorScale3D (Math|Vector|MakeVector (- (Variables|Default|Getscale) (* DeltaSeconds 1e+01)) (- (Variables|Default|Getscale) (* DeltaSeconds 1e+01)) 7e+03))
        (Variables|Default|Setscale (- (Variables|Default|Getscale) (* DeltaSeconds 1e+01)))
        (if (< (Variables|Default|Getscale) 0.0)
          (Actor|DestroyActor)))
      (else
        (Variables|Default|SetbDelay true)))
    (else
      (bind _output_get_2 (Variables|Default|SetdecreaseDelayCurrTime (+ DeltaSeconds (Variables|Default|GetdecreaseDelayCurrTime))))
      (if (> _output_get_2 (Variables|Default|GetdecreaseDelayTime))
        (Variables|Default|SetbDelay false)
        (Variables|Default|SetdecreaseDelayCurrTime 0.0)
        (Variables|Default|SetnextDelayTime (- (Variables|Default|GetnextDelayTime) (Variables|Default|GetNextDecreaseTermTime)))))))

(fn ConstructionScript)