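; BP_EnemySpawnManager is an enemy placement manager whose scatter logic is disconnected, so it currently does nothing.
; The unwired chain gathers all BP_NewEnemy actors, requires InGameMode, then runs a line trace per enemy from high to low over a hard-coded map area.
; On a hit it moves the enemy to the impact point.
; Start and end XY are randomized separately, so traces are slanted.
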(event EventBeginPlay)

(fn ConstructionScript)